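; Player controller for the FPS simulator that owns the client-side UI for players and admin spectators.
; On remote clients it creates the HUD, minimap, scoreboard, pause menu, kill cam and end screen, switching visibility and input mode on death, respawn, pause, restart and match-state changes.
; Background blur and hit effects are dynamic post-process materials blended onto the pawn's camera.
; Post-match, non-admins get the end screen, scoreboard and end-round sequence.
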(event `self.ReceiveBeginPlay`
  (bind _returnvalue (`self.K2_GetPawn`))
  (bind (_returnvalue_roll _returnvalue_pitch _returnvalue_yaw) (`KismetMathLibrary.BreakRotator` (`self.K2_GetActorRotation` _returnvalue)))
  (`/Engine/EditorBlueprintResources/ActorMacros.Switch Has Authority`
    (:`Remote`
      (`|ExecutionSequence`
        (:`then_0`
          (`self.InitHUD`)
          (`self.SetControlRotation` (`KismetMathLibrary.MakeRotator` 0.0 0.0 _returnvalue_yaw))
          (cast `/Game/Blueprints/FPSSimulatorCharacter_BP` _returnvalue
            (:`then`
              (`self.InitPlayerHUD`)
              (add `self.OnMinimapSizeUpdatedDelegate` (`|CreateDelegate` :!event `UpdateMinimapSize`))
              (add `self.OnMinimapZoomLevelUpdatedDelegate` (`|CreateDelegate` :!event `UpdateMinimapZoom`)))
            (:`CastFailed`
              (cast `/Game/Blueprints/FPSSimulatorSpectatorPawn_BP` _returnvalue)
              (set `self.bIsAdmin` true)
              (`self.InitAdminHUD`))))
        (:`then_1`
          (add `self.UIBlurMaskInitedDelegate` (`|CreateDelegate` :!event `UIBlurMaskInited`))
          (bind _asfpssimulator_game_state (cast `FPSSimulatorGameState` (`GameplayStatics.GetGameState`)))
          (bind _output_get (set `self.GameState` _asfpssimulator_game_state))
          (add `FPSSimulatorGameState.OnStateChanged` _output_get (`|CreateDelegate` :!event `OnStateChanged`))
          (if (`self.IsLocalPlayerController`)
            (`self.OnInitHUD`)))
        (:`then_2`
          (`WidgetBlueprintLibrary.SetInputMode_GameOnly` self))))))

(event `self.ReceiveTick`
  (params (DeltaSeconds :type "Float (single-precision)"))
  (bind (_returnvalue_roll _returnvalue_pitch _returnvalue_yaw) (`KismetMathLibrary.BreakRotator` (`self.GetControlRotation`)))
  (bind _hud (`self.HUD`))
  (bind _minimapmap (`/Game/Blueprints/UI/HUD/Minimap.MinimapMap` (`/Game/Blueprints/UI/HUD/HUD.Minimap` _hud)))
  (`/Engine/EditorBlueprintResources/StandardMacros.IsValid` _hud
    (:`Is Valid`
      (`/Engine/EditorBlueprintResources/StandardMacros.IsValid` _minimapmap
        (:`Is Valid`
          (`MaterialInstanceDynamic.SetScalarParameterValue` _minimapmap "Rotation" (`KismetMathLibrary.DegreesToRadians` (+ _returnvalue_yaw 90.0)))
          (`MaterialInstanceDynamic.SetVectorParameterValue` _minimapmap "Position" (`KismetMathLibrary.Conv_VectorToLinearColor` (`self.K2_GetActorLocation` (`self.K2_GetPawn`)))))))))

(event `self.DebugMessage`
  (params (Message :type String))
  (bind _asgame_mode_hud_demo (cast `/Game/Blueprints/UI/HUD/GameModeHUDs/GameModeHUD_Demo` (`self.GameModeHUD`)))
  (`/Game/Blueprints/UI/HUD/GameModeHUDs/GameModeHUD_Demo.DisplayDebugMessage` _asgame_mode_hud_demo Message))

(event `self.FlushDebugInfo`
  (`KismetSystemLibrary.FlushPersistentDebugLines`)
  (bind _asgame_mode_hud_demo (cast `/Game/Blueprints/UI/HUD/GameModeHUDs/GameModeHUD_Demo` (`self.GameModeHUD`)))
  (`/Game/Blueprints/UI/HUD/GameModeHUDs/GameModeHUD_Demo.FlushDebugMessages` _asgame_mode_hud_demo))

(event `UIBlurMaskInited`
  (bind _returnvalue (`self.K2_GetPawn`))
  (bind _returnvalue_2 (`self.K2_GetPawn`))
  (`|ExecutionSequence`
    (:`then_0`
      (`/Engine/EditorBlueprintResources/StandardMacros.IsValid` (`self.UIBlur`)
        (:`Is Valid`
          (if (`self.bIsAdmin`)
            (bind _asfpssimulator_spectator_pawn_bp (cast `/Game/Blueprints/FPSSimulatorSpectatorPawn_BP` _returnvalue_2))
            (bind _camera (`/Game/Blueprints/FPSSimulatorSpectatorPawn_BP.Camera` _asfpssimulator_spectator_pawn_bp))
            (`CameraComponent.AddOrUpdateBlendable` _camera (`self.UIBlur`) 0.0)
            (`CameraComponent.AddOrUpdateBlendable` _camera (`self.HitEffect`) 0.0)
            (else
              (bind _asfpssimulator_character_bp (cast `/Game/Blueprints/FPSSimulatorCharacter_BP` _returnvalue_2))
              (bind _camera_2 (`/Game/Blueprints/FPSSimulatorCharacter_BP.Camera` _asfpssimulator_character_bp))
              (`CameraComponent.AddOrUpdateBlendable` _camera_2 (`self.UIBlur`) 0.0)
              (`CameraComponent.AddOrUpdateBlendable` _camera_2 (`self.HitEffect`) 0.0))))))
    (:`then_1`
      (bind _returnvalue_3 (`KismetMaterialLibrary.CreateDynamicMaterialInstance` "/Game/Materials/UI/blur/UI_blur_Inst.UI_blur_Inst"))
      (bind _output_get (set `self.UIBlur` _returnvalue_3))
      (`MaterialInstanceDynamic.SetTextureParameterValue` _output_get "AlphaMask" (`DynamicTextureManager.Texture` (`self.UIBlurAlphaMask`)))
      (`MaterialInstanceDynamic.SetTextureParameterValue` _output_get "Color" (`DynamicTextureManager.Texture` (`self.UIBlurColor`)))
      (if (`self.bIsAdmin`)
        (bind _asfpssimulator_spectator_pawn_bp_2 (cast `/Game/Blueprints/FPSSimulatorSpectatorPawn_BP` _returnvalue))
        (bind _camera_3 (`/Game/Blueprints/FPSSimulatorSpectatorPawn_BP.Camera` _asfpssimulator_spectator_pawn_bp_2))
        (`CameraComponent.AddOrUpdateBlendable` _camera_3 (`self.UIBlur`) 1.0)
        (bind _returnvalue_4 (`KismetMaterialLibrary.CreateDynamicMaterialInstance` "/Game/Materials/UI/HitEffect_Inst.HitEffect_Inst"))
        (bind _output_get_2 (set `self.HitEffect` _returnvalue_4))
        (`CameraComponent.AddOrUpdateBlendable` _camera_3 _output_get_2 1.0)
        (else
          (bind _asfpssimulator_character_bp_2 (cast `/Game/Blueprints/FPSSimulatorCharacter_BP` _returnvalue))
          (bind _camera_4 (`/Game/Blueprints/FPSSimulatorCharacter_BP.Camera` _asfpssimulator_character_bp_2))
          (`CameraComponent.AddOrUpdateBlendable` _camera_4 (`self.UIBlur`) 1.0)
          (bind _returnvalue_5 (`KismetMaterialLibrary.CreateDynamicMaterialInstance` "/Game/Materials/UI/HitEffect_Inst.HitEffect_Inst"))
          (bind _output_get_3 (set `self.HitEffect` _returnvalue_5))
          (`CameraComponent.AddOrUpdateBlendable` _camera_4 _output_get_3 1.0))))))

(event `self.OnDied`
  (params (Killer :type "FPSSimulatorCharacter Object Reference"))
  (`parent.OnDied` Killer)
  (`self.SetUIVisibility` "Collapsed" true true false true true)
  (`/Game/Blueprints/UI/HUD/KillCam.SetKiller` (`self.KillCam`) Killer)
  (`self.SetUIVisibility` "Visible" false false true))

(event `self.OnRespawned`
  (`parent.OnRespawned`)
  (`self.SetUIVisibility` "Collapsed" false false true)
  (`self.SetUIVisibility` "Visible" true true)
  (`WidgetBlueprintLibrary.SetInputMode_GameOnly` self)
  (set `self.bShowMouseCursor` false))

(event `self.OnRestart_BP`
  (params (bRestart :type Boolean))
  (bind _gamestate (`self.GameState`))
  (bind ((`Map` _map) (`GameMode` _gamemode)) (break `MatchConfig` (`FPSSimulatorGameState.NextMatchConfig` _gamestate)))
  (bind ((`Map` _map_2) (`GameMode` _gamemode_2)) (break `MatchConfig` (`FPSSimulatorGameState.MatchConfig` _gamestate)))
  (`self.SetUIVisibility` "Collapsed" false false false true true)
  (bind _returnvalue (`|CreateWidget` "/Game/Blueprints/UI/LoadingScreen.LoadingScreen_C" self))
  (if bRestart
    (`/Game/Blueprints/UI/LoadingScreen.SetBG` _returnvalue (`self.GetLoadingScreenBG` _map_2 _gamemode_2))
    (else
      (`/Game/Blueprints/UI/LoadingScreen.SetBG` _returnvalue (`self.GetLoadingScreenBG` _map _gamemode))))
  (`UserWidget.AddToViewport` _returnvalue 0)
  (`WidgetBlueprintLibrary.SetInputMode_UIOnlyEx` self _returnvalue))

(event `self.ShowScoreboard`
  (`self.SetUIVisibility` "Collapsed" true true)
  (`self.SetUIVisibility` "Visible" false false false false true)
  (`self.ToggledScoreboard` true))

(event `self.HideScoreboard`
  (`self.SetUIVisibility` "Visible" true true)
  (`self.SetUIVisibility` "Collapsed" false false false false true)
  (`self.ToggledScoreboard` false))

(event `self.TogglePauseMenu`
  (bind _pausemenu (`self.PauseMenu`))
  (switch `ESlateVisibility` (`Widget.GetVisibility` (`self.PauseMenu`))
    (:`Visible`
      (`self.SetUIVisibility` "Collapsed" false false false true)
      (switch `EMatchState` (`FPSSimulatorGameState.State` (`self.GameState`))
        (:`InProgress`
          (`self.SetUIVisibility` "Visible" true true))
        (:`PostMatch`
          (`self.SetUIVisibility` "Visible" true :!label _label)
          (`self.ShowPostMatchStatus`))
        (:`PostMatchCountdown`
          (goto _label)))
      (`WidgetBlueprintLibrary.SetInputMode_GameOnly` self)
      (set `self.bShowMouseCursor` false)
      (`self.ToggledPauseMenu` true))
    (:`Collapsed`
      (`self.SetUIVisibility` "Visible" false false false true)
      (`self.SetUIVisibility` "Collapsed" true true true false true)
      (switch `EMatchState` (`FPSSimulatorGameState.State` (`self.GameState`))
        (:`InProgress`
          (`WidgetBlueprintLibrary.SetInputMode_UIOnlyEx` self _pausemenu)
          (set `self.bShowMouseCursor` true))
        (:`PostMatch`
          (`Widget.SetVisibility` (`self.PostMatchStatus`) "Collapsed" :!label _label_2)
          (`WidgetBlueprintLibrary.SetInputMode_GameAndUIEx` self _pausemenu "DoNotLock" false))
        (:`PostMatchCountdown`
          (goto _label_2)))
      (`self.ToggledPauseMenu` false))))

(event `OnStateChanged`
  (params (NewState :type "EMatchState Enum"))
  (bind _scoreboard (`self.Scoreboard`))
  (bind _endscreen (`self.EndScreen`))
  (bind _widgetswitcher (`/Game/Blueprints/UI/EndScreen.WidgetSwitcher` (`self.EndScreen`)))
  (switch `EMatchState` NewState
    (:`PostMatch`
      (`|ExecutionSequence`
        (:`then_0`
          (if (not (`self.bIsAdmin`))
            (`|ExecutionSequence`
              (:`then_0`
                (`|ExecutionSequence` :!label _label_3
                  (:`then_0`
                    (`Widget.RemoveFromParent` (`self.HUD`))
                    (`self.HideScoreboard`))
                  (:`then_1`
                    (if (`|EnumEquality` (`Widget.GetVisibility` (`self.PauseMenu`)) "Visible")
                      (`self.TogglePauseMenu`)))
                  (:`then_2`
                    (`UserWidget.AddToViewport` _endscreen 0)
                    (`WidgetBlueprintLibrary.SetInputMode_UIOnlyEx` self _endscreen)
                    (set `self.bShowMouseCursor` true))
                  (:`then_3`
                    (`/Game/Blueprints/UI/HUD/Scoreboard.ShowReadyButton` (`self.Scoreboard`)))))
              (:`then_1`
                (if (not (`PanelWidget.HasChild` _widgetswitcher _scoreboard)) :!label _label_4
                  (`PanelWidget.AddChild` _widgetswitcher _scoreboard)
                  (`Widget.SetVisibility` _scoreboard "Visible")))
              (:`then_2`
                (bind _returnvalue (`LevelSequencePlayer.CreateLevelSequencePlayer` (`FPSSimulatorGameState.EndRoundSequence` (`self.GameState`)) :!label _label_5))
                (bind _output_get (set `self.EndRoundSequencePlayer` _returnvalue))
                (`LevelSequencePlayer.Play` _output_get)))))
        (:`then_1`
          (`/Game/Blueprints/UI/HUD/Scoreboard.ShowReadyStatus` (`self.Scoreboard`) :!label _label_6)
          (`self.ShowPostMatchStatus`))))
    (:`PostMatchCountdown`
      (`|ExecutionSequence`
        (:`then_0`
          (if (not (`self.bIsAdmin`))
            (`|ExecutionSequence`
              (:`then_0`
                (if (`Widget.IsInViewport` (`self.HUD`))
                  (goto _label_3)))
              (:`then_1`
                (goto _label_4))
              (:`then_2`
                (if (`.bSkipMOS` (break `MatchConfig` (`FPSSimulatorGameState.MatchConfig` (`self.GameState`))))
                  (goto _label_5))))))
        (:`then_1`
          (goto _label_6))))))

(event `OnQOE_Submitted`
  (`WidgetSwitcher.SetActiveWidget` (`/Game/Blueprints/UI/EndScreen.WidgetSwitcher` (`self.EndScreen`)) (`self.Scoreboard`)))

(fn `GetLoadingScreenBG`
  (params (Map :type String) (GameMode :type String))
  (returns (BG :type "Texture2D Object Reference"))
  (switch `string` Map
    (:`MP_Metro`
      (switch `string` GameMode
        (:`TDM`
          (return (`WidgetBlueprintLibrary.GetBrushResourceAsTexture2D` (`WidgetBlueprintLibrary.MakeBrushFromTexture` "/Game/Textures/UI/loading_screen_Metro_TDM.loading_screen_Metro_TDM"))))
        (:`Domination`
          (return (`WidgetBlueprintLibrary.GetBrushResourceAsTexture2D` (`WidgetBlueprintLibrary.MakeBrushFromTexture` "/Game/Textures/UI/loading_screen_Metro_domination.loading_screen_Metro_domination"))))
        (:`CTF`
          (return (`WidgetBlueprintLibrary.GetBrushResourceAsTexture2D` (`WidgetBlueprintLibrary.MakeBrushFromTexture` "/Game/Textures/UI/loading_screen_Metro_CTF.loading_screen_Metro_CTF"))))))))

(fn `InitAdminHUD`
  (`|ExecutionSequence`
    (:`then_0`
      (bind _returnvalue (`|CreateWidget` "/Game/Blueprints/UI/settings/AdminSettings.AdminSettings_C" self))
      (set `self.AdminHUD` _returnvalue))
    (:`then_1`
      (`Widget.SetVisibility` (`/Game/Blueprints/UI/HUD/HUD.PersonalInfo` (`self.HUD`)) "Collapsed")
      (`Widget.SetVisibility` (`/Game/Blueprints/UI/HUD/HUD.Crosshair` (`self.HUD`)) "Collapsed"))))

(fn `InitHUD`
  (`|ExecutionSequence`
    (:`then_0`
      (bind _asfpssimulator_hud_bp (cast `/Game/Blueprints/FPSSimulatorHUD_BP` (`self.GetHUD`)))
      (set `self.GameModeHUD` (`FPSSimulatorHUD.GameModeHUD` _asfpssimulator_hud_bp)))
    (:`then_1`
      (bind _returnvalue (`|CreateWidget` "/Game/Blueprints/UI/HUD/HUD.HUD_C" self))
      (bind _output_get (set `self.HUD` _returnvalue))
      (`UserWidget.AddToViewport` _output_get 0)
      (`self.UpdateMinimapSize`))
    (:`then_2`
      (bind _returnvalue_2 (`|CreateWidget` "/Game/Blueprints/UI/HUD/Scoreboard.Scoreboard_C" self))
      (bind _output_get_2 (set `self.Scoreboard` _returnvalue_2))
      (`UserWidget.AddToViewport` _output_get_2 0)
      (`Widget.SetVisibility` _output_get_2 "Collapsed"))
    (:`then_3`
      (bind _returnvalue_3 (`|CreateWidget` "/Game/Blueprints/UI/PauseMenu.PauseMenu_C" self))
      (bind _output_get_3 (set `self.PauseMenu` _returnvalue_3))
      (`UserWidget.AddToViewport` _output_get_3 1)
      (`Widget.SetVisibility` _output_get_3 "Collapsed"))
    (:`then_4`
      (bind _returnvalue_4 (`|CreateWidget` "/Game/Blueprints/UI/PostMatchStatus.PostMatchStatus_C" self))
      (bind _output_get_4 (set `self.PostMatchStatus` _returnvalue_4))
      (`UserWidget.AddToViewport` _output_get_4 1)
      (`Widget.SetVisibility` _output_get_4 "Collapsed"))))

(fn `InitPlayerHUD`
  (`|ExecutionSequence`
    (:`then_0`
      (bind _returnvalue (`|CreateWidget` "/Game/Blueprints/UI/HUD/KillCam.KillCam_C" self))
      (bind _output_get (set `self.KillCam` _returnvalue))
      (`UserWidget.AddToViewport` _output_get 0)
      (`Widget.SetVisibility` _output_get "Collapsed"))
    (:`then_1`
      (bind _returnvalue_2 (`|CreateWidget` "/Game/Blueprints/UI/EndScreen.EndScreen_C" self))
      (bind _output_get_2 (set `self.EndScreen` _returnvalue_2))
      (add `/Game/Blueprints/UI/QOE.OnQOE_Submitted` (`/Game/Blueprints/UI/EndScreen.QOE` _output_get_2) (`|CreateDelegate` :!event `OnQOE_Submitted`)))))

(fn `SetUIVisibility`
  (params (Visible :type "ESlateVisibility Enum") (HUD :type Boolean) (GameModeHUD :type Boolean) (KillCam :type Boolean) (PauseMenu :type Boolean) (Scoreboard :type Boolean))
  (locals (bVisible :type Boolean))
  (bind _hud (`self.HUD`))
  (bind _killcam (`self.KillCam`))
  (bind _scoreboard (`self.Scoreboard`))
  (bind _pausemenu (`self.PauseMenu`))
  (bind _gamemodehud (`self.GameModeHUD`))
  (bind _output_get (set `local.bVisible` (and (`|EnumInequality` Visible "Collapsed") (`|EnumInequality` Visible "Hidden"))))
  (`|ExecutionSequence`
    (:`then_0`
      (if HUD
        (`/Engine/EditorBlueprintResources/StandardMacros.IsValid` _hud
          (:`Is Valid`
            (`Widget.SetVisibility` _hud Visible)
            (`/Game/Blueprints/UI/elements/Blur.Toggle` (`/Game/Blueprints/UI/HUD/HUD.MinimapBlurBG` _hud) _output_get)
            (`/Game/Blueprints/UI/elements/Blur.Toggle` (`/Game/Blueprints/UI/HUD/HUD.PersonalInfoBlurRect` _hud) _output_get)
            (`/Game/Blueprints/UI/elements/Blur.Toggle` (`/Game/Blueprints/UI/HUD/HUD.PersonalInfoBlurCircle` _hud) _output_get)))))
    (:`then_1`
      (if GameModeHUD
        (`/Engine/EditorBlueprintResources/StandardMacros.IsValid` _gamemodehud
          (:`Is Valid`
            (`Widget.SetVisibility` _gamemodehud Visible)))))
    (:`then_2`
      (if KillCam
        (`/Engine/EditorBlueprintResources/StandardMacros.IsValid` _killcam
          (:`Is Valid`
            (`Widget.SetVisibility` _killcam Visible)
            (`/Game/Blueprints/UI/elements/Blur.Toggle` (`/Game/Blueprints/UI/HUD/KillCam.BlurBG1` _killcam) _output_get)
            (`/Game/Blueprints/UI/elements/Blur.Toggle` (`/Game/Blueprints/UI/HUD/KillCam.BlurBG2` _killcam) _output_get)))))
    (:`then_3`
      (if PauseMenu
        (`Widget.SetVisibility` _pausemenu Visible)
        (`/Game/Blueprints/UI/elements/Blur.Toggle` (`/Game/Blueprints/UI/PauseMenu.Blur` _pausemenu) _output_get)))
    (:`then_4`
      (if Scoreboard
        (`Widget.SetVisibility` _scoreboard Visible)
        (`/Game/Blueprints/UI/elements/Blur.Toggle` (`/Game/Blueprints/UI/HUD/Scoreboard.Blur` _scoreboard) _output_get)))))

(fn `ShowPostMatchStatus`
  (`Widget.SetVisibility` (`self.PostMatchStatus`) "SelfHitTestInvisible"))

(fn `UpdateMinimapSize`
  (`/Game/Blueprints/UI/HUD/HUD.SetMinimapSize` (`self.HUD`) (`KismetMathLibrary.Conv_IntToDouble` (`self.MinimapSize`))))

(fn `UpdateMinimapZoom`
  (`/Game/Blueprints/UI/HUD/Minimap.SetZoomLevel` (`/Game/Blueprints/UI/HUD/HUD.Minimap` (`self.HUD`)) (`self.MinimapZoomLevel`)))

(fn `UserConstructionScript`)