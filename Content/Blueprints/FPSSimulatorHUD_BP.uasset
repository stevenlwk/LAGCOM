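; FPSSimulatorHUD_BP is a HUD Blueprint that passes kill feed entries to the HUD object held by the owning player controller.
; On BeginPlay it caches the HUD reference from FPSSimulatorPlayerController_BP, or binds to the controller's OnInitHUD dispatcher to cache it once initialized.
; ShowKillEntry forwards killer, victim and weapon to that object's AddKillFeed, without a validity check.
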(event `self.ReceiveBeginPlay`
  (bind _asfpssimulator_player_controller_bp (cast `/Game/Blueprints/FPSSimulatorPlayerController_BP` (`self.GetOwningPlayerController`)))
  (bind _hud (`/Game/Blueprints/FPSSimulatorPlayerController_BP.HUD` _asfpssimulator_player_controller_bp))
  (`/Engine/EditorBlueprintResources/StandardMacros.IsValid` _hud
    (:`Is Valid`
      (set `self.HUD` _hud))
    (:`Is Not Valid`
      (add `/Game/Blueprints/FPSSimulatorPlayerController_BP.OnInitHUD` _asfpssimulator_player_controller_bp (delegate `OnInitHUD`)))))

(event `OnInitHUD`
  (bind _asfpssimulator_player_controller_bp (cast `/Game/Blueprints/FPSSimulatorPlayerController_BP` (`self.GetOwningPlayerController`)))
  (set `self.HUD` (`/Game/Blueprints/FPSSimulatorPlayerController_BP.HUD` _asfpssimulator_player_controller_bp)))

(fn `ShowKillEntry`
  (params (Killer :type "FPSSimulatorCharacter Object Reference") (Victim :type "FPSSimulatorCharacter Object Reference") (Weapon :type "BaseWeapon Object Reference"))
  (`/Game/Blueprints/UI/HUD/HUD.AddKillFeed` (`self.HUD`) Killer Victim Weapon))

(fn `UserConstructionScript`)