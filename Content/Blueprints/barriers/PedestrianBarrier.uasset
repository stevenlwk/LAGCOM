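; Spline-driven pedestrian barrier actor that lays out fence pieces as mesh instances in the construction script, with no runtime logic.
; It walks an optionally closed spline by accumulated distance, alternating connectors and full barrier sections while they fit, then adds a closing connector.
; Optional small sections cap the start and end.
; A helper supplies each piece's location and rotation from its distance and length, with scale fixed.
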(event EventBeginPlay)

(event Collision|EventActorBeginOverlap
  (params (OtherActor :type Actor%20Object%20Reference)))

(event EventTick
  (params (DeltaSeconds :type Float%20%28single-precision%29)))

(fn ConstructionScript
  (bind _smalllength (Variables|Default|GetSmallLength))
  (bind (_location _rotation) (Utilities|GetTransformatDistanceAlongSpline 0.0 _smalllength))
  (Utilities|FlowControl|Sequence
    (:then_0
      (Spline|SetClosedLoop (Variables|Default|GetSpline) (Variables|Default|GetClosedLoop)))
    (:then_1
      (if (Variables|Default|GetSmallStart)
        (Components|InstancedStaticMesh|AddInstance (Variables|Default|GetPedestrianBarrierSmall) (Math|Transform|MakeTransform _location _rotation "1,1,1"))
        (LocalVariables|SetDistance (+ (LocalVariables|GetDistance) (Variables|Default|GetSmallLength)))))
    (:then_2
      (while (< (+ (LocalVariables|GetDistance) (Variables|Default|GetConnectorLength) (Variables|Default|GetLength)) (Spline|GetSplineLength (Variables|Default|GetSpline)))
        (Components|InstancedStaticMesh|AddInstance (Variables|Default|GetPedestrianBarrierConnector) (Math|Transform|MakeTransform (.Location (Utilities|GetTransformatDistanceAlongSpline (LocalVariables|GetDistance) (Variables|Default|GetConnectorLength))) (.Rotation (Utilities|GetTransformatDistanceAlongSpline (LocalVariables|GetDistance) (Variables|Default|GetConnectorLength))) "1,1,1"))
        (bind _output_get (LocalVariables|SetDistance (+ (LocalVariables|GetDistance) (Variables|Default|GetConnectorLength))))
        (Components|InstancedStaticMesh|AddInstance (Variables|Default|GetPedestrianBarrier) (Math|Transform|MakeTransform (.Location (Utilities|GetTransformatDistanceAlongSpline _output_get (Variables|Default|GetLength))) (.Rotation (Utilities|GetTransformatDistanceAlongSpline _output_get (Variables|Default|GetLength))) "1,1,1"))
        (LocalVariables|SetDistance (+ (LocalVariables|GetDistance) (Variables|Default|GetLength)))))
    (:then_3
      (Components|InstancedStaticMesh|AddInstance (Variables|Default|GetPedestrianBarrierConnector) (Math|Transform|MakeTransform (.Location (Utilities|GetTransformatDistanceAlongSpline (LocalVariables|GetDistance) (Variables|Default|GetConnectorLength))) (.Rotation (Utilities|GetTransformatDistanceAlongSpline (LocalVariables|GetDistance) (Variables|Default|GetConnectorLength))) "1,1,1"))
      (LocalVariables|SetDistance (+ (LocalVariables|GetDistance) (Variables|Default|GetConnectorLength))))
    (:then_4
      (if (Variables|Default|GetSmallEnd)
        (Components|InstancedStaticMesh|AddInstance (Variables|Default|GetPedestrianBarrierSmall) (Math|Transform|MakeTransform (.Location (Utilities|GetTransformatDistanceAlongSpline (LocalVariables|GetDistance) (Variables|Default|GetSmallLength))) (.Rotation (Utilities|GetTransformatDistanceAlongSpline (LocalVariables|GetDistance) (Variables|Default|GetSmallLength))) "1,1,1"))))))