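; Spline-based concrete barrier actor that lays out rows of instanced barrier meshes at construction time.
; The construction script steps along the spline by segment length, spawning at a configurable interval and offset and stacking copies into layers by height.
; Each instance faces the next spline point, but its Z comes only from the layer, ignoring spline height.
; An optional flag applies a fixed cull distance to the instances.
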(fn `UserConstructionScript`
  (bind _spline (`self.Spline`))
  (`|ExecutionSequence`
    (:`then_0`
      (if (`self.Cull`)
        (`InstancedStaticMeshComponent.SetCullDistances` (`self.ConcreteBarrier`) 6000 6000)))
    (:`then_1`
      (for _index (range (+ (`.ReturnValue` (`KismetMathLibrary.FMod` (`SplineComponent.GetSplineLength` _spline) (`self.Length`))) 1))
        (if (== (mod (+ _index (`self.Offset`)) (`self.SpawnEvery`)) 0)
          (for _index_2 (range (`self.NumLayers`))
            (bind _returnvalue (* _index (`self.Length`)))
            (bind (_returnvalue_x _returnvalue_y _returnvalue_z) (`KismetMathLibrary.BreakVector` (`SplineComponent.GetLocationAtDistanceAlongSpline` _spline _returnvalue "Local")))
            (`InstancedStaticMeshComponent.AddInstance` (`self.ConcreteBarrier`) (`KismetMathLibrary.MakeTransform` (`KismetMathLibrary.MakeVector` _returnvalue_x _returnvalue_y (* _index_2 (`self.Height`))) (`KismetMathLibrary.Conv_VectorToRotator` (- (`SplineComponent.GetLocationAtDistanceAlongSpline` _spline (+ _returnvalue (`self.Length`)) "Local") (`KismetMathLibrary.MakeVector` _returnvalue_x _returnvalue_y _returnvalue_z)))))))))))