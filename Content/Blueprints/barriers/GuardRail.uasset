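; GuardRail is a barrier actor that lines a spline with repeated guard rail segments.
; The Construction Script divides the spline length by the segment Length and adds one GuardRail mesh instance at each step.
; Each instance is aimed along the straight chord to the next step point in local space, keeping unit scale rather than bending to the curve.
; The event graph has no active logic.
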(event `self.ReceiveBeginPlay`)

(event `self.ReceiveActorBeginOverlap`
  (params (OtherActor :type "Actor Object Reference")))

(event `self.ReceiveTick`
  (params (DeltaSeconds :type "Float (single-precision)")))

(fn `UserConstructionScript`
  (bind _spline (`self.Spline`))
  (for _index (range (+ (`.ReturnValue` (`KismetMathLibrary.FMod` (`SplineComponent.GetSplineLength` _spline) (`self.Length`))) 1))
    (bind _returnvalue (* _index (`self.Length`)))
    (bind _returnvalue_2 (`SplineComponent.GetLocationAtDistanceAlongSpline` _spline _returnvalue "Local"))
    (`InstancedStaticMeshComponent.AddInstance` (`self.GuardRail`) (`KismetMathLibrary.MakeTransform` _returnvalue_2 (`KismetMathLibrary.Conv_VectorToRotator` (- (`SplineComponent.GetLocationAtDistanceAlongSpline` _spline (+ _returnvalue (`self.Length`)) "Local") _returnvalue_2))))))