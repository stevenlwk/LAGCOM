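; Spline-driven blueprint that lays out a row of crowd control barriers along an editable path.
; The construction script steps along the spline at Length intervals, adding an unscaled mesh instance in local space at each step.
; Each instance is rotated toward the next sample point, so segments follow the curve as straight chords.
; The event graph holds no active logic.
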(event EventBeginPlay)

(event Collision|EventActorBeginOverlap
  (params (OtherActor :type Actor%20Object%20Reference)))

(event EventTick
  (params (DeltaSeconds :type Float%20%28single-precision%29)))

(fn ConstructionScript
  (bind _spline (Variables|Default|GetSpline))
  (while (< (LocalVariables|GetDistance) (Spline|GetSplineLength _spline))
    (Components|InstancedStaticMesh|AddInstance (Variables|Default|GetCrowdControlBarrier) (Math|Transform|MakeTransform (Spline|GetLocationatDistanceAlongSpline _spline (LocalVariables|GetDistance) "Local") (Math|Conversions|RotationFromXVector (- (Spline|GetLocationatDistanceAlongSpline _spline (+ (LocalVariables|GetDistance) (Variables|Default|GetLength)) "Local") (Spline|GetLocationatDistanceAlongSpline _spline (LocalVariables|GetDistance) "Local"))) "1,1,1"))
    (LocalVariables|SetDistance (+ (LocalVariables|GetDistance) (Variables|Default|GetLength)))))