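; Player character Blueprint for a team-based FPS, handling the cosmetic response to character events.
; On clients, BeginPlay caches game state and local player references, binds fire and invincibility events, and adds minimap icons and beacons for non-local characters.
; Timelines drive ADS FOV, crouch camera height and hit post-processing through a material parameter collection.
; It also swaps team materials, spawns first- or third-person weapons by local control, and feeds hit indicators and kill feed.
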(event `self.ReceiveBeginPlay`
  (`/Engine/EditorBlueprintResources/ActorMacros.Switch Has Authority`
    (:`Remote`
      (`|ExecutionSequence`
        (:`then_0`
          (switch `int` (`self.TeamID`)
            (:`0`
              (`self.OnRep_TeamID`))))
        (:`then_1`
          (bind _asfpssimulator_game_state (cast `FPSSimulatorGameState` (`GameplayStatics.GetGameState`)))
          (set `self.GameState` _asfpssimulator_game_state))
        (:`then_2`
          (bind _asfpssimulator_player_controller_bp (cast `/Game/Blueprints/FPSSimulatorPlayerController_BP` (`GameplayStatics.GetPlayerController` 0)))
          (bind _output_get (set `self.LocalPC` _asfpssimulator_player_controller_bp))
          (bind _asfpssimulator_character (cast `FPSSimulatorCharacter` (`Controller.K2_GetPawn` _output_get)))
          (set `self.LocalCharacter` _asfpssimulator_character)
          (`/Engine/EditorBlueprintResources/StandardMacros.IsValid` (`/Game/Blueprints/FPSSimulatorPlayerController_BP.HUD` _output_get)
            (:`Is Valid`
              (`self.OnInitHUD`))
            (:`Is Not Valid`
              (add `/Game/Blueprints/FPSSimulatorPlayerController_BP.OnInitHUD` _output_get (`|CreateDelegate` :!event `OnInitHUD`)))))
        (:`then_3`
          (add `self.OnFireDelegate` (`|CreateDelegate` :!event `OnFire`))
          (add `self.OnStartInvincibilityDelegate` (`|CreateDelegate` :!event `OnStartInvincibility`))
          (add `self.OnEndInvincibilityDelegate` (`|CreateDelegate` :!event `OnEndInvincibility`)))))))

(event `self.OnADSStarted`
  (`self.ShowCrosshair` false)
  (bind (_direction _alpha) (`Timeline|ADS` :!label _label)
    (:`Update`
      (set `self.ADSBlend` _alpha)
      (set `CameraComponent.FieldOfView` (`KismetMathLibrary.Lerp` 90.0 60.0 _alpha) (`self.Camera`)))))

(event `self.OnADSEnded`
  (`self.ShowCrosshair` true)
  (goto _label :!via `Reverse`))

(event `self.OnConfirmHit_BP`
  (params (HitFrom :type "Vector Structure"))
  (`|ExecutionSequence`
    (:`then_0`
      (bind (_direction _intensity) (`Timeline|HitEffectTimeline` :!via `PlayFromStart`)
        (:`Update`
          (`KismetMaterialLibrary.SetScalarParameterValue` "/Game/Materials/UI/HitEffectParameterCollection.HitEffectParameterCollection" "BlurWidth" (* (`self.MaxHitBlurWidth`) _intensity))
          (`KismetMaterialLibrary.SetScalarParameterValue` "/Game/Materials/UI/HitEffectParameterCollection.HitEffectParameterCollection" "VignetteIntensity" (* (`self.MaxHitVignetteIntensity`) _intensity))
          (`KismetMaterialLibrary.SetScalarParameterValue` "/Game/Materials/UI/HitEffectParameterCollection.HitEffectParameterCollection" "DesaturationIntensity" (* (`self.MaxHitDesaturationPercentage`) _intensity)))))
    (:`then_1`
      (bind _returnvalue (`|CreateWidget` "/Game/Blueprints/UI/HUD/HitIndicator.HitIndicator_C" (`self.LocalPC`)))
      (set `/Game/Blueprints/UI/HUD/HitIndicator.ShotLocation` HitFrom _returnvalue)
      (`Overlay.AddChildToOverlay` (`/Game/Blueprints/UI/HUD/HUD.HitIndicators` (`self.HUD`)) _returnvalue))))

(event `OnFire` :!signature `self.OnFireDelegate`
  (params (HitResult :type "HitResult Structure"))
  (`GameplayStatics.SpawnEmitterAtLocation` "/Game/Particles/P_Sparks.P_Sparks" HitResult_Location (struct))
  (`GameplayStatics.PlaySoundAtLocation` "/Game/Sounds/weapons/M4A1/M4A1_single_SoundCue.M4A1_single_SoundCue" (`SceneComponent.K2_GetComponentLocation` (`self.MuzzleSocket`))))

(event `self.OnDied_BP`
  (params (Killer :type "FPSSimulatorCharacter Object Reference"))
  (`|ExecutionSequence`
    (:`then_0`
      (if (`self.IsLocallyControlled`)
        (`SceneComponent.SetHiddenInGame` (`self.FP_Mesh`) true true)))
    (:`then_1`
      (bind _asfpssimulator_player_controller_bp (cast `/Game/Blueprints/FPSSimulatorPlayerController_BP` (`GameplayStatics.GetPlayerController` 0)))
      (bind _asfpssimulator_hud_bp (cast `/Game/Blueprints/FPSSimulatorHUD_BP` (`PlayerController.GetHUD` _asfpssimulator_player_controller_bp)))
      (`/Game/Blueprints/FPSSimulatorHUD_BP.ShowKillEntry` _asfpssimulator_hud_bp Killer self (`FPSSimulatorCharacter.Weapon` Killer)))))

(event `OnInitHUD`
  (bind _minimap (`/Game/Blueprints/UI/HUD/HUD.Minimap` (`self.HUD`)))
  (bind _item (`KismetArrayLibrary.Array_Get` (`FPSSimulatorGameState.TeamColors` (`self.GameState`)) (`self.TeamID`)))
  (`/Engine/EditorBlueprintResources/ActorMacros.Switch Has Authority`
    (:`Remote`
      (`|ExecutionSequence`
        (:`then_0`
          (set `self.HUD` (`/Game/Blueprints/FPSSimulatorPlayerController_BP.HUD` (`self.LocalPC`))))
        (:`then_1`
          (if (not (`self.IsLocallyControlled`))
            (`|ExecutionSequence`
              (:`then_0`
                (if (== (`FPSSimulatorCharacter.TeamID` (`self.LocalCharacter`)) (`self.TeamID`))
                  (bind _icon (`/Game/Blueprints/UI/HUD/Minimap.AddIcon` _minimap "/Game/Blueprints/UI/elements/Icons/PlayerIconDirectional.PlayerIconDirectional_C" self 0))
                  (`/Game/Blueprints/UI/elements/Icons/Icon.SetColor` _icon _item)
                  (else
                    (bind _icon_2 (`/Game/Blueprints/UI/HUD/Minimap.AddIcon` _minimap "/Game/Blueprints/UI/elements/Icons/PlayerIcon.PlayerIcon_C" self 0))
                    (`/Game/Blueprints/UI/elements/Icons/Icon.SetColor` _icon_2 _item))))
              (:`then_1`
                (bind _beacon (`/Game/Blueprints/UI/HUD/HUD.AddBeacon` (`self.HUD`) "/Game/Blueprints/UI/elements/Beacons/PlayerBeacon.PlayerBeacon_C" self 0))
                (bind _asplayer_beacon (cast `/Game/Blueprints/UI/elements/Beacons/PlayerBeacon` _beacon))
                (`/Game/Blueprints/UI/elements/Beacons/PlayerBeacon.SetPlayer` _asplayer_beacon self)))))))))

(event `self.OnRep_TeamID`
  (bind _mesh (`self.Mesh`))
  (switch `int` (`self.TeamID`)
    (:`0`
      (`PrimitiveComponent.SetMaterial` _mesh 0 "/Game/Characters/Materials/BotBodyBlue.BotBodyBlue")
      (`PrimitiveComponent.SetMaterial` (`self.FP_Mesh`) 0 "/Game/Characters/Materials/BotBodyBlue.BotBodyBlue")
      (`PrimitiveComponent.SetMaterial` _mesh 1 "/Game/Characters/Materials/BotBodyBlueJoints.BotBodyBlueJoints")
      (`PrimitiveComponent.SetMaterial` (`self.FP_Mesh`) 1 "/Game/Characters/Materials/BotBodyBlueJoints.BotBodyBlueJoints"))
    (:`1`
      (`PrimitiveComponent.SetMaterial` _mesh 0 "/Game/Characters/Materials/BotBodyRed.BotBodyRed")
      (`PrimitiveComponent.SetMaterial` (`self.FP_Mesh`) 0 "/Game/Characters/Materials/BotBodyRed.BotBodyRed")
      (`PrimitiveComponent.SetMaterial` _mesh 1 "/Game/Characters/Materials/BotBodyRedJoints.BotBodyRedJoints")
      (`PrimitiveComponent.SetMaterial` (`self.FP_Mesh`) 1 "/Game/Characters/Materials/BotBodyRedJoints.BotBodyRedJoints"))))

(event `self.OnRespawned`
  (`SceneComponent.SetHiddenInGame` (`self.FP_Mesh`) false true))

(event `self.OnRunningStarted`
  (`self.ShowCrosshair` false))

(event `self.OnRunningEnded`
  (`self.ShowCrosshair` true))

(event `self.K2_OnStartCrouch`
  (params (HalfHeightAdjust :type "Float (single-precision)") (ScaledHalfHeightAdjust :type "Float (single-precision)"))
  (bind _camera (`self.Camera`))
  (bind (_relativelocation_x _relativelocation_y) (`KismetMathLibrary.BreakVector` (`SceneComponent.RelativeLocation` _camera)))
  (bind (_direction _cameraz) (`Timeline|CameraCrouch` :!label _label_2)
    (:`Update`
      (`SceneComponent.K2_SetRelativeLocation` _camera (`KismetMathLibrary.MakeVector` _relativelocation_x _relativelocation_y _cameraz) false false))))

(event `self.K2_OnEndCrouch`
  (params (HalfHeightAdjust :type "Float (single-precision)") (ScaledHalfHeightAdjust :type "Float (single-precision)"))
  (goto _label_2 :!via `Reverse`))

(event `OnStartInvincibility`
  (bind _mesh (`self.Mesh`))
  (switch `int` (`self.TeamID`)
    (:`0`
      (`PrimitiveComponent.SetMaterial` _mesh 0 "/Game/Characters/Materials/InvincibleBotBodyBlue.InvincibleBotBodyBlue")
      (`PrimitiveComponent.SetMaterial` (`self.FP_Mesh`) 0 "/Game/Characters/Materials/InvincibleBotBodyBlue.InvincibleBotBodyBlue"))
    (:`1`
      (`PrimitiveComponent.SetMaterial` _mesh 0 "/Game/Characters/Materials/InvincibleBotBodyRed.InvincibleBotBodyRed")
      (`PrimitiveComponent.SetMaterial` (`self.FP_Mesh`) 0 "/Game/Characters/Materials/InvincibleBotBodyRed.InvincibleBotBodyRed"))))

(event `OnEndInvincibility`
  (bind _mesh (`self.Mesh`))
  (switch `int` (`self.TeamID`)
    (:`0`
      (`PrimitiveComponent.SetMaterial` _mesh 0 "/Game/Characters/Materials/BotBodyBlue.BotBodyBlue")
      (`PrimitiveComponent.SetMaterial` (`self.FP_Mesh`) 0 "/Game/Characters/Materials/BotBodyBlue.BotBodyBlue"))
    (:`1`
      (`PrimitiveComponent.SetMaterial` _mesh 0 "/Game/Characters/Materials/BotBodyRed.BotBodyRed")
      (`PrimitiveComponent.SetMaterial` (`self.FP_Mesh`) 0 "/Game/Characters/Materials/BotBodyRed.BotBodyRed"))))

(event `self.ShowHitMarker_BP`
  (bind _asfpssimulator_player_controller_bp (cast `/Game/Blueprints/FPSSimulatorPlayerController_BP` (`self.GetController`)))
  (`/Game/Blueprints/UI/HUD/HUD.ShowHitMarker` (`/Game/Blueprints/FPSSimulatorPlayerController_BP.HUD` _asfpssimulator_player_controller_bp)))

(event `self.SetWeapon`
  (bind _tp_weapon (`self.TP_Weapon`))
  (bind _fp_weapon (`self.FP_Weapon`))
  (if (`self.IsLocallyControlled`)
    (`ChildActorComponent.SetChildActorClass` _fp_weapon (`self.WeaponClass`))
    (bind _asbase_weapon_bp (cast `/Game/Blueprints/weapon/BaseWeapon_BP` (`ChildActorComponent.ChildActor` _fp_weapon)))
    (`PrimitiveComponent.SetCastShadow` (`/Game/Blueprints/weapon/BaseWeapon_BP.WeaponMesh` _asbase_weapon_bp) false)
    (set `self.HandguardSocket` (`/Game/Blueprints/weapon/BaseWeapon_BP.HandguardSocket` _asbase_weapon_bp))
    (set `self.SightSocket` (`/Game/Blueprints/weapon/BaseWeapon_BP.SightSocket` _asbase_weapon_bp))
    (set `self.MuzzleSocket` (`/Game/Blueprints/weapon/BaseWeapon_BP.MuzzleSocket` _asbase_weapon_bp))
    (`self.OnSetWeapon`)
    (else
      (`SceneComponent.SetHiddenInGame` (`self.FP_Mesh`) true true)
      (`ChildActorComponent.SetChildActorClass` _tp_weapon (`self.WeaponClass`))
      (bind _asbase_weapon_bp_2 (cast `/Game/Blueprints/weapon/BaseWeapon_BP` (`ChildActorComponent.ChildActor` _tp_weapon)))
      (set `self.HandguardSocket` (`/Game/Blueprints/weapon/BaseWeapon_BP.HandguardSocket` _asbase_weapon_bp_2))
      (set `self.MuzzleSocket` (`/Game/Blueprints/weapon/BaseWeapon_BP.MuzzleSocket` _asbase_weapon_bp_2))
      (`self.OnSetWeapon`))))

(event `self.OnWeaponFireModeChanged`
  (`GameplayStatics.SpawnSoundAttached` "/Game/Sounds/weapons/M4A1/M4A1_switch_Cue.M4A1_switch_Cue" (`self.Mesh`) "Weapon"))

(fn `UserConstructionScript`)