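; CTF_Base_BP is a capture-the-flag team base that shows a border around its area on clients.
; On remote BeginPlay, if the game state is GS_CTF, it sizes the Border widget component from the Area box extents and passes the TeamID to its CTF_BaseBorder widget.
; Outside CTF, the actor hides itself on the client.
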(event `self.ReceiveBeginPlay`
  (bind _border (`self.Border`))
  (bind (_boxextent_x _boxextent_y) (`KismetMathLibrary.BreakVector` (`BoxComponent.BoxExtent` (`self.Area`))))
  (`/Engine/EditorBlueprintResources/ActorMacros.Switch Has Authority`
    (:`Remote`
      (cast `GS_CTF` (`GameplayStatics.GetGameState`)
        (:`then`
          (`WidgetComponent.SetDrawSize` _border (`KismetMathLibrary.MakeVector2D` (* _boxextent_y 2.0) (* _boxextent_x 2.0)))
          (bind _asctf_base_border (cast `/Game/Blueprints/UI/CTF_BaseBorder` (`WidgetComponent.GetUserWidgetObject` _border)))
          (`/Game/Blueprints/UI/CTF_BaseBorder.SetTeam` _asctf_base_border (`self.TeamID`)))
        (:`CastFailed`
          (`self.SetActorHiddenInGame` true))))))

(fn `UserConstructionScript`)