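; Game state for the Domination mode that sets up capture point HUD elements on remote clients only.
; On BeginPlay, and again when the player controller fires OnInitHUD, it registers every capture point with the Domination HUD and adds a minimap icon and beacon for each.
; It also listens for match state changes, removing the mode HUD during post-match countdown and post-match.
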(event `self.ReceiveBeginPlay`
  (bind _hud (`/Game/Blueprints/FPSSimulatorPlayerController_BP.HUD` (`self.PC`)))
  (bind _hud_2 (`/Game/Blueprints/FPSSimulatorPlayerController_BP.HUD` (`self.PC`)))
  (`/Engine/EditorBlueprintResources/ActorMacros.Switch Has Authority`
    (:`Remote`
      (`|ExecutionSequence`
        (:`then_0`
          (add `self.OnStateChanged` (`|CreateDelegate` :!event `OnStateChanged_BP`))
          (bind _asfpssimulator_player_controller_bp (cast `/Game/Blueprints/FPSSimulatorPlayerController_BP` (`GameplayStatics.GetPlayerController` 0)))
          (bind _output_get (set `self.PC` _asfpssimulator_player_controller_bp))
          (add `/Game/Blueprints/FPSSimulatorPlayerController_BP.OnInitHUD` _output_get (`|CreateDelegate` :!event `OnInitHUD`)))
        (:`then_1`
          (`|ExecutionSequence` :!label _label
            (:`then_0`
              (bind _asgame_mode_hud_domination (cast `/Game/Blueprints/UI/HUD/GameModeHUDs/GameModeHUD_Domination` (`/Game/Blueprints/FPSSimulatorPlayerController_BP.GameModeHUD` (`self.PC`))))
              (set `self.GameModeHUD` _asgame_mode_hud_domination))
            (:`then_1`
              (bind _outactors (`GameplayStatics.GetAllActorsOfClass` "/Game/Blueprints/CapturePoint_BP.CapturePoint_BP_C"))
              (for _array_element _outactors
                (`|ExecutionSequence`
                  (:`then_0`
                    (`/Game/Blueprints/UI/HUD/GameModeHUDs/GameModeHUD_Domination.AddCapturePoint` (`self.GameModeHUD`) _array_element))
                  (:`then_1`
                    (`/Engine/EditorBlueprintResources/StandardMacros.IsValid` _hud_2
                      (:`Is Valid`
                        (bind _icon (`/Game/Blueprints/UI/HUD/Minimap.AddIcon` (`/Game/Blueprints/UI/HUD/HUD.Minimap` _hud_2) "/Game/Blueprints/UI/elements/Icons/CapturePointIcon.CapturePointIcon_C" _array_element -1))
                        (bind _ascapture_point_icon (cast `/Game/Blueprints/UI/elements/Icons/CapturePointIcon` _icon))
                        (`/Game/Blueprints/UI/elements/Icons/CapturePointIcon.SetCapturePoint` _ascapture_point_icon _array_element))))
                  (:`then_2`
                    (`/Engine/EditorBlueprintResources/StandardMacros.IsValid` _hud
                      (:`Is Valid`
                        (bind _beacon (`/Game/Blueprints/UI/HUD/HUD.AddBeacon` _hud "/Game/Blueprints/UI/elements/Beacons/CapturePointBeacon.CapturePointBeacon_C" _array_element 0))
                        (bind _ascapture_point_beacon (cast `/Game/Blueprints/UI/elements/Beacons/CapturePointBeacon` _beacon))
                        (`/Game/Blueprints/UI/elements/Beacons/CapturePointBeacon.SetCapturePoint` _ascapture_point_beacon _array_element)))))))))))))

(event `OnInitHUD`
  (goto _label))

(event `OnStateChanged_BP` :!signature `self.OnStateChanged`
  (params (NewState :type "EMatchState Enum"))
  (bind _gamemodehud (`self.GameModeHUD`))
  (switch `EMatchState` NewState
    (:`PostMatch`
      _)
    (:`PostMatchCountdown`
      _))
  (`/Engine/EditorBlueprintResources/StandardMacros.IsValid` _gamemodehud
    (:`Is Valid`
      (`Widget.RemoveFromParent` _gamemodehud))))

(fn `UserConstructionScript`)