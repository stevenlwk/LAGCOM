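; Capture the Flag game state that, on remote clients only, manages the mode's minimap icons and HUD beacons.
; On BeginPlay and again on HUD init, it caches the CTF HUD and adds an icon and beacon for every base.
; Flag spawns add the same markers, storing beacons by team ID so flag returns can remove them.
; Post-match states remove the CTF HUD.
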(event `self.ReceiveBeginPlay`
  (bind _hud (`/Game/Blueprints/FPSSimulatorPlayerController_BP.HUD` (`self.PC`)))
  (`/Engine/EditorBlueprintResources/ActorMacros.Switch Has Authority`
    (:`Remote`
      (`|ExecutionSequence`
        (:`then_0`
          (bind _asfpssimulator_player_controller_bp (cast `/Game/Blueprints/FPSSimulatorPlayerController_BP` (`GameplayStatics.GetPlayerController` 0)))
          (bind _output_get (set `self.PC` _asfpssimulator_player_controller_bp))
          (add `/Game/Blueprints/FPSSimulatorPlayerController_BP.OnInitHUD` _output_get (`|CreateDelegate` :!event `OnInitHUD`)))
        (:`then_1`
          (add `self.OnFlagSpawnedDelegate` (`|CreateDelegate` :!event `OnFlagSpawned_BP`))
          (add `self.OnFlagReturnedDelegate` (`|CreateDelegate` :!event `OnFlagReturned_BP`))
          (add `self.OnStateChanged` (`|CreateDelegate` :!event `OnStateChanged_BP`)))
        (:`then_2`
          (`|ExecutionSequence` :!label _label
            (:`then_0`
              (bind _asgame_mode_hud_ctf (cast `/Game/Blueprints/UI/HUD/GameModeHUDs/GameModeHUD_CTF` (`/Game/Blueprints/FPSSimulatorPlayerController_BP.GameModeHUD` (`self.PC`))))
              (set `self.GameModeHUD` _asgame_mode_hud_ctf))
            (:`then_1`
              (`/Engine/EditorBlueprintResources/StandardMacros.IsValid` _hud
                (:`Is Valid`
                  (bind _outactors (`GameplayStatics.GetAllActorsOfClass` "/Game/Blueprints/CTF_Base_BP.CTF_Base_BP_C"))
                  (for _array_element _outactors
                    (`|ExecutionSequence`
                      (:`then_0`
                        (bind _icon (`/Game/Blueprints/UI/HUD/Minimap.AddIcon` (`/Game/Blueprints/UI/HUD/HUD.Minimap` _hud) "/Game/Blueprints/UI/elements/Icons/CTF_BaseIcon.CTF_BaseIcon_C" _array_element -1))
                        (bind _asctf_base_icon (cast `/Game/Blueprints/UI/elements/Icons/CTF_BaseIcon` _icon))
                        (`/Game/Blueprints/UI/elements/Icons/CTF_BaseIcon.SetBase` _asctf_base_icon _array_element))
                      (:`then_1`
                        (bind _beacon (`/Game/Blueprints/UI/HUD/HUD.AddBeacon` _hud "/Game/Blueprints/UI/elements/Beacons/CTF_BaseBeacon.CTF_BaseBeacon_C" _array_element 0))
                        (bind _asctf_base_beacon (cast `/Game/Blueprints/UI/elements/Beacons/CTF_BaseBeacon` _beacon))
                        (`/Game/Blueprints/UI/elements/Beacons/CTF_BaseBeacon.SetBase` _asctf_base_beacon _array_element)))))))))))))

(event `OnInitHUD`
  (goto _label))

(event `OnStateChanged_BP` :!signature `self.OnStateChanged`
  (params (NewState :type "EMatchState Enum"))
  (bind _gamemodehud (`self.GameModeHUD`))
  (switch `EMatchState` NewState
    (:`PostMatch`
      _)
    (:`PostMatchCountdown`
      _))
  (`/Engine/EditorBlueprintResources/StandardMacros.IsValid` _gamemodehud
    (:`Is Valid`
      (`Widget.RemoveFromParent` _gamemodehud))))

(event `OnFlagSpawned_BP` :!signature `self.OnFlagSpawnedDelegate`
  (params (Flag :type "CTF_Flag Object Reference"))
  (bind _hud (`/Game/Blueprints/FPSSimulatorPlayerController_BP.HUD` (`self.PC`)))
  (`/Engine/EditorBlueprintResources/StandardMacros.IsValid` _hud
    (:`Is Valid`
      (`|ExecutionSequence`
        (:`then_0`
          (bind _icon (`/Game/Blueprints/UI/HUD/Minimap.AddIcon` (`/Game/Blueprints/UI/HUD/HUD.Minimap` _hud) "/Game/Blueprints/UI/elements/Icons/CTF_FlagIcon.CTF_FlagIcon_C" Flag -1))
          (bind _asctf_flag_icon (cast `/Game/Blueprints/UI/elements/Icons/CTF_FlagIcon` _icon))
          (bind _asctf_flag_bp (cast `/Game/Blueprints/CTF_Flag_BP` Flag))
          (`/Game/Blueprints/UI/elements/Icons/CTF_FlagIcon.SetFlag` _asctf_flag_icon _asctf_flag_bp))
        (:`then_1`
          (bind _beacon (`/Game/Blueprints/UI/HUD/HUD.AddBeacon` _hud "/Game/Blueprints/UI/elements/Beacons/CTF_FlagBeacon.CTF_FlagBeacon_C" Flag 0))
          (bind _asctf_flag_beacon (cast `/Game/Blueprints/UI/elements/Beacons/CTF_FlagBeacon` _beacon))
          (`KismetArrayLibrary.Array_Set` (`self.Beacons`) (`CTF_Flag.TeamID` Flag) _asctf_flag_beacon true)
          (`/Game/Blueprints/UI/elements/Beacons/CTF_FlagBeacon.SetFlag` _asctf_flag_beacon _asctf_flag_bp))))))

(event `OnFlagReturned_BP` :!signature `self.OnFlagReturnedDelegate`
  (params (Flag :type "CTF_Flag Object Reference"))
  (`Widget.RemoveFromParent` (`KismetArrayLibrary.Array_Get` (`self.Beacons`) (`CTF_Flag.TeamID` Flag))))

(fn `UserConstructionScript`)