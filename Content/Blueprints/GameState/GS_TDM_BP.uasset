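; Team Deathmatch game state that manages the client-side lifetime of the mode's HUD widget.
; On remote instances only, BeginPlay binds to state changes and caches the local FPS simulator player controller.
; It fetches that controller's TDM HUD immediately and again on OnInitHUD, covering late HUD creation.
; When the state becomes Post Match or Post Match Countdown, it removes the HUD from its parent.
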(event `self.ReceiveBeginPlay`
  (`/Engine/EditorBlueprintResources/ActorMacros.Switch Has Authority`
    (:`Remote`
      (`|ExecutionSequence`
        (:`then_0`
          (add `self.OnStateChanged` (`|CreateDelegate` :!event `OnStateChanged_BP`))
          (bind _asfpssimulator_player_controller_bp (cast `/Game/Blueprints/FPSSimulatorPlayerController_BP` (`GameplayStatics.GetPlayerController` 0)))
          (bind _output_get (set `self.PC` _asfpssimulator_player_controller_bp))
          (add `/Game/Blueprints/FPSSimulatorPlayerController_BP.OnInitHUD` _output_get (`|CreateDelegate` :!event `OnInitHUD`)))
        (:`then_1`
          (bind _asgame_mode_hud_tdm (cast `/Game/Blueprints/UI/HUD/GameModeHUDs/GameModeHUD_TDM` (`/Game/Blueprints/FPSSimulatorPlayerController_BP.GameModeHUD` (`self.PC`)) :!label _label))
          (set `self.GameModeHUD` _asgame_mode_hud_tdm))))))

(event `OnInitHUD`
  (goto _label))

(event `OnStateChanged_BP` :!signature `self.OnStateChanged`
  (params (NewState :type "EMatchState Enum"))
  (bind _gamemodehud (`self.GameModeHUD`))
  (switch `EMatchState` NewState
    (:`PostMatch`
      _)
    (:`PostMatchCountdown`
      _))
  (`/Engine/EditorBlueprintResources/StandardMacros.IsValid` _gamemodehud
    (:`Is Valid`
      (`Widget.RemoveFromParent` _gamemodehud))))

(fn `UserConstructionScript`)