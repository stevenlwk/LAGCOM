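; Metro escalator Blueprint that builds its row of steps at construction time from a four-point Path spline.
; The construction script walks along local X from a StepOffset-shifted start, alternating instances between the StepA and StepB instanced meshes.
; Horizontal spacing is StepLength on the landings and eases tighter on the incline between the middle points.
; FindZ sets each step's height, flat on both landings and linearly interpolated along the slope.
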(fn `FindZ`
  (params (X :type "Float (double-precision)"))
  (returns (Z :type "Float (double-precision)"))
  (locals (p1 :type "Vector Structure") (p2 :type "Vector Structure"))
  (bind _path (`self.path`))
  (bind (_p1_x _p1_y _p1_z) (`KismetMathLibrary.BreakVector` (`local.p1`)))
  (bind (_p2_x _p2_y _p2_z) (`KismetMathLibrary.BreakVector` (`local.p2`)))
  (bind (_p1_x_2 _p1_y_2 _p1_z_2) (`KismetMathLibrary.BreakVector` (`local.p1`)))
  (bind (_p2_x_2 _p2_y_2 _p2_z_2) (`KismetMathLibrary.BreakVector` (`local.p2`)))
  (`|ExecutionSequence`
    (:`then_0`
      (set `local.p1` (`SplineComponent.GetLocationAtSplinePoint` _path 1 "Local"))
      (set `local.p2` (`SplineComponent.GetLocationAtSplinePoint` _path 2 "Local")))
    (:`then_1`
      (if (<= X _p1_x)
        (return _p1_z)
        (elif (>= X _p2_x)
          (return _p2_z)
          (else
            (return (`KismetMathLibrary.MapRangeUnclamped` X _p1_x_2 _p2_x_2 _p1_z_2 _p2_z_2))))))))

(fn `UserConstructionScript`
  (locals (stepLength :type "Float (double-precision)" :default 34.0) (lastX :type "Float (double-precision)"))
  (bind _path (`self.path`))
  (bind _lastx (`local.lastX`))
  (bind _returnvalue_x (`KismetMathLibrary.BreakVector` (`SplineComponent.GetLocationAtSplinePoint` _path 1 "Local")))
  (bind _returnvalue_x_2 (`KismetMathLibrary.BreakVector` (`SplineComponent.GetLocationAtSplinePoint` (`self.path`) 0 "Local")))
  (bind _returnvalue_x_3 (`KismetMathLibrary.BreakVector` (`SplineComponent.GetLocationAtSplinePoint` (`self.path`) 3 "Local")))
  (bind _z (`self.FindZ` _lastx))
  (bind _returnvalue_x_4 (`KismetMathLibrary.BreakVector` (`SplineComponent.GetLocationAtSplinePoint` _path 2 "Local")))
  (bind _returnvalue (+ (`local.lastX`) (`local.stepLength`)))
  (bind _returnvalue_2 (+ (`local.lastX`) (`local.stepLength`)))
  (set `local.lastX` (- (+ _returnvalue_x_2 (* (`local.stepLength`) (`self.stepOffset`))) (`local.stepLength`)))
  (while (< (`local.lastX`) _returnvalue_x_3)
    (if (not (`KismetMathLibrary.InRange_FloatFloat` _returnvalue_2 _returnvalue_x _returnvalue_x_4 false false))
      (set `local.lastX` _returnvalue_2)
      (else
        (set `local.lastX` (+ (`local.lastX`) (`KismetMathLibrary.MapRangeClamped` (`KismetMathLibrary.FMin` (- _returnvalue _returnvalue_x) (- (+ _returnvalue_x_4 (`local.stepLength`)) _returnvalue)) 0.0 34.0 34.0 32.0)))))
    (`/Engine/EditorBlueprintResources/StandardMacros.FlipFlop`
      (:`A`
        (`InstancedStaticMeshComponent.AddInstance` (`self.step a`) (`KismetMathLibrary.MakeTransform` (`KismetMathLibrary.MakeVector` _lastx 0.0 _z))))
      (:`B`
        (`InstancedStaticMeshComponent.AddInstance` (`self.step b`) (`KismetMathLibrary.MakeTransform` (`KismetMathLibrary.MakeVector` _lastx 0.0 _z)))))))