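; Metro rail Blueprint that builds a straight two-rail track with a length set by NumRails.
; The construction script adds paired Rail mesh instances either side of the local Y axis, roughly standard gauge apart.
; Pairs repeat every 10 m along negative Y, starting from a half-length offset so the track straddles the actor origin.
; The event graph holds only disabled stubs, so there is no runtime logic.
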(fn `UserConstructionScript`
  (locals (HalfLength :type "Float (double-precision)"))
  (bind _rail (`self.rail`))
  (set `local.HalfLength` (* (`self.NumRails`) 500.0))
  (for _index (range (`self.NumRails`))
    (bind _returnvalue (+ (* _index -1000.0) (`local.HalfLength`)))
    (`InstancedStaticMeshComponent.AddInstance` _rail (`KismetMathLibrary.MakeTransform` (`KismetMathLibrary.MakeVector` -71.75 _returnvalue)))
    (`InstancedStaticMeshComponent.AddInstance` _rail (`KismetMathLibrary.MakeTransform` (`KismetMathLibrary.MakeVector` 71.75 _returnvalue)))))