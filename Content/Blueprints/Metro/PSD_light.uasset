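; PSD_light is a Metro Blueprint that builds an evenly spaced row of point lights along its local X axis.
; Its construction script derives the repeat pitch and half the total row length from the light count, segment length and gap length.
; It then loops to add one point light component per segment, subtracting half the row length and adding HalfLength to center the row on the actor.
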(fn `UserConstructionScript`
  (locals (HalfTotalLength :type "Float (double-precision)") (RepeatLength :type "Float (double-precision)") (HalfLength :type "Float (double-precision)" :default 95.0))
  (bind _numlights (`self.NumLights`))
  (set `local.RepeatLength` (+ (`self.Length`) (`self.GapLength`)))
  (set `local.HalfTotalLength` (/ (+ (* _numlights (`self.Length`)) (* (- _numlights 1) (`self.GapLength`))) 2.0))
  (for _index (range (`self.NumLights`))
    (`AddComponent|NODE_AddPointLightComponent-10` :`RelativeTransform` (`KismetMathLibrary.MakeTransform` (`KismetMathLibrary.MakeVector` (+ (- (* _index (`local.RepeatLength`)) (`local.HalfTotalLength`)) (`local.HalfLength`))) (struct) (1.0 1.0 1.0)))))