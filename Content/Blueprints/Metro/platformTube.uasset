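; Metro platform Blueprint that procedurally builds a grid of tube meshes in its construction script.
; It adds instances to the Tube component, with rows along X and columns along Y, spaced by tube size plus gaps.
; Listed row indices are either skipped or squashed to half length, with an optional mirror flag shifting half tubes to the other end of their cell.
; The component is finally offset to center the columns on Y.
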(fn `UserConstructionScript`
  (locals (InnerRowGap :type "Float (double-precision)" :default 5.67) (TubeWidth :type "Float (double-precision)" :default 4.33) (TubeLength :type "Float (double-precision)" :default 115.0) (InnerColumnGap :type "Float (double-precision)" :default 7.5))
  (bind _numcolumns (`self.NumColumns`))
  (bind _tube (`self.tube`))
  (for _index (range (`self.NumTubes`))
    (if (== (`KismetArrayLibrary.Array_Find` (`self.TubesToSkip`) _index) -1)
      (for _index_2 (range (`self.NumColumns`))
        (if (== (`KismetArrayLibrary.Array_Find` (`self.HalfTubes`) _index) -1)
          (bind _returnvalue (* _index (+ (`local.TubeWidth`) (`local.InnerRowGap`))))
          (bind _returnvalue_2 (* _index_2 (+ (`local.TubeLength`) (`local.InnerColumnGap`))))
          (`InstancedStaticMeshComponent.AddInstance` _tube (`KismetMathLibrary.MakeTransform` (`KismetMathLibrary.MakeVector` _returnvalue _returnvalue_2)))
          (elif (`self.MirrorHalfTubes`)
            (`InstancedStaticMeshComponent.AddInstance` _tube (`KismetMathLibrary.MakeTransform` (`KismetMathLibrary.MakeVector` _returnvalue (+ _returnvalue_2 (/ (`local.TubeLength`) 2.0))) (struct) (1.0 0.5 1.0)))
            (else
              (`InstancedStaticMeshComponent.AddInstance` _tube (`KismetMathLibrary.MakeTransform` (`KismetMathLibrary.MakeVector` _returnvalue _returnvalue_2) (struct) (1.0 0.5 1.0)))))))))
  (`SceneComponent.K2_AddLocalOffset` (`self.tube`) (`KismetMathLibrary.MakeVector` 0.0 (- 0.0 (/ (+ (* _numcolumns (`local.TubeLength`)) (* (- _numcolumns 1) (`local.InnerColumnGap`))) 2.0))) false false))