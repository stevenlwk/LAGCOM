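; Metro concourse construction script that procedurally lays out a field of tubes and two runs of panels as instanced components.
; Tubes repeat along X at width-plus-gap spacing in each column Y position, skipping five consecutive slots in every 28, shifted by LightOffset, apparently leaving openings for lights.
; Both panel components receive matching instances stepped along Y by panel length.
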(fn `UserConstructionScript`
  (locals (InnerRowGap :type "Float (double-precision)" :default 5.67) (TubeWidth :type "Float (double-precision)" :default 4.33) (PanelLength :type "Float (double-precision)" :default 240.0))
  (`|ExecutionSequence`
    (:`then_0`
      (for _array_element (`self.tubeColumnY`)
        (for _index (range (`self.NumTubes`))
          (if (not (<= (mod (+ _index (`self.lightOffset`)) 28) 4))
            (`InstancedStaticMeshComponent.AddInstance` (`self.tube`) (`KismetMathLibrary.MakeTransform` (`KismetMathLibrary.MakeVector` (* _index (+ (`local.TubeWidth`) (`local.InnerRowGap`))) _array_element)))))))
    (:`then_1`
      (for _index_2 (range (`self.numPanels`))
        (bind _returnvalue (* _index_2 (`local.PanelLength`)))
        (`InstancedStaticMeshComponent.AddInstance` (`self.panel`) (`KismetMathLibrary.MakeTransform` (`KismetMathLibrary.MakeVector` 0.0 _returnvalue)))
        (`InstancedStaticMeshComponent.AddInstance` (`self.panel2`) (`KismetMathLibrary.MakeTransform` (`KismetMathLibrary.MakeVector` 0.0 _returnvalue)))))))