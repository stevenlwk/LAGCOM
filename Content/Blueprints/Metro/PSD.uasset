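; Metro platform screen door (PSD) wall, built procedurally from a door count and centred on the actor.
; The construction script alternates fixed panel and door instances with matching glass, adding end panels and choosing board variants by platform number and door parity.
; At runtime it listens to the player controller's planar reflection level, making the glass smooth for Large Only or All and rough otherwise.
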(event `self.ReceiveBeginPlay`
  (bind _asfpssimulator_player_controller (cast `FPSSimulatorPlayerController` (`GameplayStatics.GetPlayerController` 0)))
  (bind _output_get (set `self.Controller` _asfpssimulator_player_controller))
  (add `FPSSimulatorPlayerController.OnPlanarReflecitonLevelUpdatedDelegate` _output_get (delegate `OnPlanarReflecitonLevelUpdated`))
  (`self.OnPlanarReflecitonLevelUpdated`))

(event `OnPlanarReflecitonLevelUpdated`
  (bind _psd1_glass (`self.PSD1_glass`))
  (switch `EPlanarReflectionLevel` (`FPSSimulatorPlayerController.PlanarReflectionLevel` (`self.Controller`))
    (:`None`
      (`MeshComponent.SetScalarParameterValueOnMaterials` _psd1_glass "Roughness" 1.0 :!label _label)
      (`MeshComponent.SetScalarParameterValueOnMaterials` (`self.PSD2b_glass`) "Roughness" 1.0)
      (`MeshComponent.SetScalarParameterValueOnMaterials` (`self.PSD2a_glass`) "Roughness" 1.0))
    (:`SmallOnly`
      (goto _label))
    (:`LargeOnly`
      (`MeshComponent.SetScalarParameterValueOnMaterials` _psd1_glass "Roughness" 0.0 :!label _label_2)
      (`MeshComponent.SetScalarParameterValueOnMaterials` (`self.PSD2b_glass`) "Roughness" 0.0)
      (`MeshComponent.SetScalarParameterValueOnMaterials` (`self.PSD2a_glass`) "Roughness" 0.0))
    (:`All`
      (goto _label_2))))

(fn `UserConstructionScript`
  (locals (PSD1Width :type "Float (double-precision)" :default 318.0) (PSD2Width :type "Float (double-precision)" :default 268.0) (HalfTotalWidth :type "Float (double-precision)") (TotalWidth :type "Float (double-precision)"))
  (bind _numdoors (`self.NumDoors`))
  (bind _returnvalue (- (`local.TotalWidth`) (`local.PSD1Width`)))
  (bind _output_get (set `local.TotalWidth` (+ (* _numdoors (`local.PSD2Width`)) (* (+ _numdoors 2) (`local.PSD1Width`)))))
  (set `local.HalfTotalWidth` (/ _output_get 2.0))
  (`InstancedStaticMeshComponent.AddInstance` (`self.PSD1`) (`KismetMathLibrary.MakeTransform` (0.0 0.0 0.0) (struct :`Yaw` 90.0)))
  (`InstancedStaticMeshComponent.AddInstance` (`self.PSD1_glass`) (`KismetMathLibrary.MakeTransform` (0.0 0.0 0.0) (struct :`Yaw` 90.0)))
  (`InstancedStaticMeshComponent.AddInstance` (`self.PSD1_board_c`) (`KismetMathLibrary.MakeTransform` (0.0 0.0 0.0) (struct :`Yaw` 90.0)))
  (for _index (range (`self.NumDoors`))
    (`|ExecutionSequence`
      (:`then_0`
        (bind _returnvalue_2 (+ (* _index (+ (`local.PSD1Width`) (`local.PSD2Width`))) (`local.PSD1Width`)))
        (`InstancedStaticMeshComponent.AddInstance` (`self.PSD2a`) (`KismetMathLibrary.MakeTransform` (`KismetMathLibrary.MakeVector` 0.0 _returnvalue_2) (struct :`Yaw` 90.0) (1.0 1.0 1.0)))
        (`InstancedStaticMeshComponent.AddInstance` (`self.PSD2a_glass`) (`KismetMathLibrary.MakeTransform` (`KismetMathLibrary.MakeVector` 0.0 _returnvalue_2) (struct :`Yaw` 90.0) (1.0 1.0 1.0))))
      (:`then_1`
        (`InstancedStaticMeshComponent.AddInstance` (`self.PSD2b`) (`KismetMathLibrary.MakeTransform` (`KismetMathLibrary.MakeVector` 0.0 _returnvalue_2) (struct :`Yaw` 90.0)))
        (`InstancedStaticMeshComponent.AddInstance` (`self.PSD2b_glass`) (`KismetMathLibrary.MakeTransform` (`KismetMathLibrary.MakeVector` 0.0 _returnvalue_2) (struct :`Yaw` 90.0))))
      (:`then_2`
        (switch `int` (mod _index 2)
          (:`0`
            (`InstancedStaticMeshComponent.AddInstance` (`self.PSD2_board_c`) (`KismetMathLibrary.MakeTransform` (`KismetMathLibrary.MakeVector` 0.0 _returnvalue_2) (struct :`Yaw` 90.0))))
          (:`1`
            (switch `int` (`self.Platform`)
              (:`1`
                (`InstancedStaticMeshComponent.AddInstance` (`self.PSD2_board_a`) (`KismetMathLibrary.MakeTransform` (`KismetMathLibrary.MakeVector` 0.0 _returnvalue_2) (struct :`Yaw` 90.0))))
              (:`2`
                (`InstancedStaticMeshComponent.AddInstance` (`self.PSD2_board_b`) (`KismetMathLibrary.MakeTransform` (`KismetMathLibrary.MakeVector` 0.0 _returnvalue_2) (struct :`Yaw` 90.0))))))))
      (:`then_3`
        (bind _returnvalue_3 (+ _returnvalue_2 (`local.PSD2Width`)))
        (`InstancedStaticMeshComponent.AddInstance` (`self.PSD1`) (`KismetMathLibrary.MakeTransform` (`KismetMathLibrary.MakeVector` 0.0 _returnvalue_3) (struct :`Yaw` 90.0)))
        (`InstancedStaticMeshComponent.AddInstance` (`self.PSD1_glass`) (`KismetMathLibrary.MakeTransform` (`KismetMathLibrary.MakeVector` 0.0 _returnvalue_3) (struct :`Yaw` 90.0))))
      (:`then_4`
        (switch `int` (`self.Platform`)
          (:`1`
            (`InstancedStaticMeshComponent.AddInstance` (`self.PSD1_board_a`) (`KismetMathLibrary.MakeTransform` (`KismetMathLibrary.MakeVector` 0.0 _returnvalue_3) (struct :`Yaw` 90.0))))
          (:`2`
            (`InstancedStaticMeshComponent.AddInstance` (`self.PSD1_board_b`) (`KismetMathLibrary.MakeTransform` (`KismetMathLibrary.MakeVector` 0.0 _returnvalue_3) (struct :`Yaw` 90.0) (1.0 1.0 1.0))))))))
  (`InstancedStaticMeshComponent.AddInstance` (`self.PSD1`) (`KismetMathLibrary.MakeTransform` (`KismetMathLibrary.MakeVector` 0.0 _returnvalue) (struct :`Yaw` 90.0)))
  (`InstancedStaticMeshComponent.AddInstance` (`self.PSD1_glass`) (`KismetMathLibrary.MakeTransform` (`KismetMathLibrary.MakeVector` 0.0 _returnvalue) (struct :`Yaw` 90.0)))
  (`InstancedStaticMeshComponent.AddInstance` (`self.PSD1_board_c`) (`KismetMathLibrary.MakeTransform` (`KismetMathLibrary.MakeVector` 0.0 _returnvalue) (struct :`Yaw` 90.0)))
  (`SceneComponent.K2_AddLocalOffset` (`self.PSD1`) (`KismetMathLibrary.MakeVector` 0.0 (- 0.0 (`local.HalfTotalWidth`))) false false)
  (`SceneComponent.K2_AddLocalOffset` (`self.PSD1_glass`) (`KismetMathLibrary.MakeVector` 0.0 (- 0.0 (`local.HalfTotalWidth`))) false false)
  (`SceneComponent.K2_AddLocalOffset` (`self.PSD1_board_c`) (`KismetMathLibrary.MakeVector` 0.0 (- 0.0 (`local.HalfTotalWidth`))) false false)
  (`SceneComponent.K2_AddLocalOffset` (`self.PSD1_board_b`) (`KismetMathLibrary.MakeVector` 0.0 (- 0.0 (`local.HalfTotalWidth`))) false false)
  (`SceneComponent.K2_AddLocalOffset` (`self.PSD1_board_a`) (`KismetMathLibrary.MakeVector` 0.0 (- 0.0 (`local.HalfTotalWidth`))) false false)
  (`SceneComponent.K2_AddLocalOffset` (`self.PSD2b`) (`KismetMathLibrary.MakeVector` 0.0 (- 0.0 (`local.HalfTotalWidth`))) false false)
  (`SceneComponent.K2_AddLocalOffset` (`self.PSD2a`) (`KismetMathLibrary.MakeVector` 0.0 (- 0.0 (`local.HalfTotalWidth`))) false false)
  (`SceneComponent.K2_AddLocalOffset` (`self.PSD2b_glass`) (`KismetMathLibrary.MakeVector` 0.0 (- 0.0 (`local.HalfTotalWidth`))) false false)
  (`SceneComponent.K2_AddLocalOffset` (`self.PSD2a_glass`) (`KismetMathLibrary.MakeVector` 0.0 (- 0.0 (`local.HalfTotalWidth`))) false false)
  (`SceneComponent.K2_AddLocalOffset` (`self.PSD2_board_c`) (`KismetMathLibrary.MakeVector` 0.0 (- 0.0 (`local.HalfTotalWidth`))) false false)
  (`SceneComponent.K2_AddLocalOffset` (`self.PSD2_board_b`) (`KismetMathLibrary.MakeVector` 0.0 (- 0.0 (`local.HalfTotalWidth`))) false false)
  (`SceneComponent.K2_AddLocalOffset` (`self.PSD2_board_a`) (`KismetMathLibrary.MakeVector` 0.0 (- 0.0 (`local.HalfTotalWidth`))) false false))